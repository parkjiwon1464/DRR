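; Game mode for the inventory system that relays chest, dropped item and actor destruction changes on the server.
; PostLogin collects every joining controller in AllPCs, with no removal on logout in this graph.
; Chest updates and ground item list refreshes loop over that array, calling each BP_InventoryPlayerController, which receives the calling PC for radius-based chest updates.
; Other events directly update a chest's slots or a dropped item's amount, or destroy a given actor.
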(event `UpdateChestGM`
  (params (Chest :type "Object Object Reference") (visibilities :type "Array of Boolean (by ref)") (items :type "Array of /Game/AdvancedInventory/Structures/Item_Structur Structure (by ref)") (PC :type "PlayerController Object Reference"))
  ;[1 0.1453 0.1354 1 142] Add this to your GameMode
  ;;[1 1 1] Update chest from the GameMode
  (bind _asbp_chest (cast `/Game/AdvancedInventory/Blueprints/BP_Chest` Chest))
  (`/Game/AdvancedInventory/Blueprints/BP_Chest.UpdateChestSlots` _asbp_chest visibilities items PC))

(event `self.K2_PostLogin`
  (params (NewPlayer :type "PlayerController Object Reference"))
  ;[1 0.1453 0.1354 1 142] Add this to your GameMode
  ;;[1 1 1] Creates an array wich contains all players on the server  (connect with "EventOnPostLogin")
  (`KismetArrayLibrary.Array_Add` (`self.All PCs`) NewPlayer))

(event `UpdateChestForPlayersWhoAreInRadiusOfTheChest`
  (params (chest :type "/Game/AdvancedInventory/Blueprints/BP_Chest Object Reference") (PC :type "PlayerController Object Reference") (visibilities :type "Array of Boolean (by ref)") (items :type "Array of /Game/AdvancedInventory/Structures/Item_Structur Structure (by ref)"))
  ;[1 0.1453 0.1354 1 142] Add this to your GameMode
  ;;[1 1 1] Update a specific chest for all players who are near to this chest, except for the player who calls the update
  (for _array_element (`self.All PCs`)
    (`/Game/AdvancedInventory/Blueprints/BP_InventoryPlayerController.UpdateWhenThsPCisInRadiusOfTheChest` (`self.getPC` _array_element) chest PC visibilities items)))

(event `UpdateAmountOfA SpecificItem`
  (params (NewParam :type "Actor Object Reference") (amount :type Integer))
  ;[1 0.1453 0.1354 1 142] Add this to your GameMode
  ;;[1 1 1] Update amount of a specific item
  (bind _asbp_drop_item_actor_master (cast `/Game/AdvancedInventory/Blueprints/BP_DropItemActor_Master` NewParam))
  (`/Game/AdvancedInventory/Blueprints/BP_DropItemActor_Master.UpdateAmount` _asbp_drop_item_actor_master amount))

(event `UpdateGroundItemListOnEachPlayer`
  ;[1 0.1453 0.1354 1 142] Add this to your GameMode
  ;;[1 1 1] Update GroundItemList on each player
  (for _array_element (`self.All PCs`)
    (`/Game/AdvancedInventory/Blueprints/BP_InventoryPlayerController.UpdateGroundItemList` (`self.getPC` _array_element))))

(event `DestroyActorFromGM`
  (params (Target :type "Actor Object Reference"))
  ;[1 0.1453 0.1354 1 142] Add this to your GameMode
  ;;[1 1 1] Destroy an actor from the GameMode
  (`self.K2_DestroyActor` Target))

(fn `getPC`
  (params (input :type "PlayerController Object Reference"))
  (returns (PC :type "/Game/AdvancedInventory/Blueprints/BP_InventoryPlayerController Object Reference"))
  (bind _asbp_inventory_player_controller (cast `/Game/AdvancedInventory/Blueprints/BP_InventoryPlayerController` input))
  (return _asbp_inventory_player_controller))

(fn `UserConstructionScript`)