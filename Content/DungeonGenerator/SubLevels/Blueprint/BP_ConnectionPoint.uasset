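; Connection point actor for dungeon generator sublevels, marking a link by compass position, level, type and state.
; The construction script labels its text render with the position initial, level and type, and colors an arrow by state: Empty, Connected, Blocked or Unused.
; BeginPlay reapplies that color, and the ChangeState event stores a new state and recolors the arrow to match.
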(event `self.ReceiveBeginPlay`
  (switch `/Game/DungeonGenerator/SubLevels/Blueprint/ConnectionPointState` (`self.State`)
    (:`NewEnumerator0`
      (`ArrowComponent.SetArrowColor` (`self.StateArrow`) (struct :`R` 1.0 :`G` 0.480464 :`A` 1.0)))
    (:`NewEnumerator1`
      (`ArrowComponent.SetArrowColor` (`self.StateArrow`) (struct :`R` 0.20558 :`G` 1.0 :`A` 1.0)))
    (:`NewEnumerator2`
      (`ArrowComponent.SetArrowColor` (`self.StateArrow`) (struct :`R` 1.0 :`G` 0.033106 :`A` 1.0)))
    (:`NewEnumerator3`
      (`ArrowComponent.SetArrowColor` (`self.StateArrow`) (struct :`R` 0.32447 :`G` 0.333333 :`B` 0.322353 :`A` 1.0)))))

(event `ChangeState`
  (params (NewState :type "/Game/DungeonGenerator/SubLevels/Blueprint/ConnectionPointState Enum" :default "NewEnumerator0"))
  (bind _output_get (set `self.State` NewState))
  (switch `/Game/DungeonGenerator/SubLevels/Blueprint/ConnectionPointState` _output_get
    (:`NewEnumerator0`
      (`ArrowComponent.SetArrowColor` (`self.StateArrow`) (struct :`R` 1.0 :`G` 0.480464 :`A` 1.0)))
    (:`NewEnumerator1`
      (`ArrowComponent.SetArrowColor` (`self.StateArrow`) (struct :`R` 0.20558 :`G` 1.0 :`A` 1.0)))
    (:`NewEnumerator2`
      (`ArrowComponent.SetArrowColor` (`self.StateArrow`) (struct :`R` 1.0 :`G` 0.033106 :`A` 1.0)))
    (:`NewEnumerator3`
      (`ArrowComponent.SetArrowColor` (`self.StateArrow`) (struct :`R` 0.32447 :`G` 0.333333 :`B` 0.322353 :`A` 1.0)))))

(fn `UserConstructionScript`
  (locals (Position :type String))
  (`TextRenderComponent.K2_SetText` (`self.TextRender`) (`|FormatText` "{Position} {Level}{Type}" (`KismetTextLibrary.Conv_TextToString` (select `/Game/DungeonGenerator/SubLevels/Blueprint/ConnectionPointPosition` (`self.Position`) :`NewEnumerator0` "N" :`NewEnumerator1` "S" :`NewEnumerator2` "E" :`NewEnumerator3` "W")) (`self.Level`) (`self.Type`)))
  (switch `/Game/DungeonGenerator/SubLevels/Blueprint/ConnectionPointState` (`self.State`)
    (:`NewEnumerator0`
      (`ArrowComponent.SetArrowColor` (`self.StateArrow`) (struct :`R` 1.0 :`G` 0.480464 :`A` 1.0)))
    (:`NewEnumerator1`
      (`ArrowComponent.SetArrowColor` (`self.StateArrow`) (struct :`R` 0.20558 :`G` 1.0 :`A` 1.0)))
    (:`NewEnumerator2`
      (`ArrowComponent.SetArrowColor` (`self.StateArrow`) (struct :`R` 1.0 :`G` 0.033106 :`A` 1.0)))
    (:`NewEnumerator3`
      (`ArrowComponent.SetArrowColor` (`self.StateArrow`) (struct :`R` 0.32447 :`G` 0.333333 :`B` 0.322353 :`A` 1.0)))))